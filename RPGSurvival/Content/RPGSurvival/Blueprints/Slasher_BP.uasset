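; Slasher enemy Blueprint that handles on-screen targeting feedback through stat and lock-on reticle widget components.
; Events push stat info to the stat widget, show or hide both widgets while toggling the reticle when visibility changes, and toggle lock-on text.
; Melee damage is a debug print placeholder.
; The construction script and animation getters for avoid, block, combat transition, fatality, player damage, roll, skills and taunts are empty stubs.
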(event `self.UpdateStats`
  (params (StatInfo :type "StatInfo Structure"))
  ;[1 1 1] Update Stat UI
  (bind _asenemy_stat_bp (cast `/Game/RPGSurvival/UI/EnemyStat_BP` (`WidgetComponent.GetUserWidgetObject` (`self.StatWidget`))))
  (`/Game/RPGSurvival/UI/EnemyStat_BP.UpdateStats` _asenemy_stat_bp StatInfo))

(event `self.ShowInformation`
  (params (Show :type Boolean))
  (bind _lockonwidget (`self.LockOnWidget`))
  ;[1 1 1] Shows the lock on widget UI.
  (if (not (== Show (`SceneComponent.bVisible` _lockonwidget)))
    (`SceneComponent.SetVisibility` _lockonwidget Show false)
    (`SceneComponent.SetVisibility` (`self.StatWidget`) Show false)
    (`/Game/RPGSurvival/UI/EnemyTargetReticle_BP.ToggleReticle` (cast `/Game/RPGSurvival/UI/EnemyTargetReticle_BP` (`WidgetComponent.GetUserWidgetObject` _lockonwidget) :!pure true))))

(event `self.ToggleLockOn`
  ;[1 1 1] Toggle lock on text.
  (`/Game/RPGSurvival/UI/EnemyTargetReticle_BP.ToggleLockOnText` (cast `/Game/RPGSurvival/UI/EnemyTargetReticle_BP` (`WidgetComponent.GetUserWidgetObject` (`self.LockOnWidget`)) :!pure true)))

(event `/Game/CloseCombat/Blueprints/Interfaces/AnimBP_Interface.DamageMelee`
  (params (DamageParameters :type "/Game/CloseCombat/Blueprints/Weapon/ParentWeapon/DamageParam_Struct Structure"))
  (`KismetSystemLibrary.PrintString` "Hello"))

(fn `GetAnim_Avoid`
  (params (Direction :type String))
  (returns (Animation :type "AnimSequence Object Reference"))
  (return null))

(fn `GetAnim_Block`
  (params (Attack :type Boolean) (Index :type Integer) (RandomAnimations :type Boolean))
  (returns (Animation :type "AnimSequence Object Reference"))
  (return null))

(fn `GetAnim_CombatTransition`
  (params (State :type String))
  (returns (Animation :type "AnimSequence Object Reference"))
  (return null))

(fn `GetAnim_Fatality`
  (params (Stealth :type Boolean) (FatalityType :type String))
  (returns (FatalityArray :type "Array of /Game/CloseCombat/Blueprints/Player/Components/Fatality_Struct Structure"))
  (return))

(fn `GetAnim_Player_Damage`
  (returns (DamageAnim :type "AnimSequenceBase Object Reference"))
  (return null))

(fn `GetAnim_Roll`
  (params (Direction :type String))
  (returns (Animation :type "AnimSequence Object Reference"))
  (return null))

(fn `GetAnim_Skills`
  (params (SkillName :type String))
  (returns (Animation :type "AnimSequence Object Reference"))
  (return null))

(fn `GetAnim_Taunts`
  (params (Index :type Integer) (RandomTaunt :type Boolean))
  (returns (Animation :type "AnimSequence Object Reference"))
  (return null))

(fn `UserConstructionScript`)